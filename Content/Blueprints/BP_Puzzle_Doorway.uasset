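; Large double doorway for a puzzle that opens when OpenDoor is called from outside.
; A Box trigger shows the player an "open door" interaction prompt and registers this door on the ThirdPersonCharacter as the nearby big door.
; OpenDoor plays a timeline that yaws both door meshes, destroys the trigger and hides the player's key mesh.
; End overlap hides the prompt and clears the proximity flag without checking which actor left.
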(event OnComponentBeginOverlap(Box)
  (params (OverlappedComponent :type Primitive%20Component%20Object%20Reference) (OtherActor :type Actor%20Object%20Reference) (OtherComp :type Primitive%20Component%20Object%20Reference) (OtherBodyIndex :type Integer) (bFromSweep :type Boolean) (SweepResult :type Hit%20Result%20Structure%20%28by%20ref%29))
  (bind _asthird_person_character (Utilities|Casting|CastToThirdPersonCharacter OtherActor))
  (Variables|Default|SetRef%20Player _asthird_person_character)
  (Default|DisplayInterWidget _asthird_person_character "open" "door")
  (Variables|/Game/Blueprints/ThirdPersonCharacter.ThirdPersonCharacter_C|SetAreWeNearBigDoor? _asthird_person_character true)
  (Variables|/Game/Blueprints/ThirdPersonCharacter.ThirdPersonCharacter_C|SetBigDoorObject _asthird_person_character self))

(event OnComponentEndOverlap(Box)
  (params (OverlappedComponent :type Primitive%20Component%20Object%20Reference) (OtherActor :type Actor%20Object%20Reference) (OtherComp :type Primitive%20Component%20Object%20Reference) (OtherBodyIndex :type Integer))
  (bind _ref_player (Variables|Default|GetRef%20Player))
  (Default|HideInterWidget _ref_player)
  (Variables|/Game/Blueprints/ThirdPersonCharacter.ThirdPersonCharacter_C|SetAreWeNearBigDoor? _ref_player false)
  (Variables|/Game/Blueprints/ThirdPersonCharacter.ThirdPersonCharacter_C|SetBigDoorObject _ref_player self))

(event Custom|OpenDoor
  (CallFunction|OpenDoorsEvent)
  (Components|DestroyComponent (Variables|Default|GetBox))
  (Development|SetHiddeninGame (Variables|/Game/Blueprints/ThirdPersonCharacter.ThirdPersonCharacter_C|GetKeyMesh (Variables|Default|GetRef%20Player)) true false))

(event Custom|OpenDoorsEvent
  (bind (_direction _door_right _door_left) (Timeline|OpenDoors Play)
    (:Update
      (Transformation|SetRelativeRotation (Variables|Default|GetSM_DoorWay_Large_Door_Right) (Math|Rotator|MakeRotator 0.0 0.0 _door_right) false false)
      (Transformation|SetRelativeRotation (Variables|Default|GetSM_DoorWay_Large_Door_Left) (Math|Rotator|MakeRotator 0.0 0.0 _door_left) false false))))

(fn ConstructionScript)