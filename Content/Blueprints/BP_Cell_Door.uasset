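; BP_Cell_Door is a cell door that prompts the player to open it and swings open on a timeline.
; Its trigger box casts to ThirdPersonCharacter, shows an "open door" prompt and sets the player's near-door flag, clearing both on exit.
; An OpenDoor event rotates the mesh's yaw through the DoorRotate timeline, destroys the trigger and hides the player's key mesh.
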(event OnComponentBeginOverlap(Box)
  (params (OverlappedComponent :type Primitive%20Component%20Object%20Reference) (OtherActor :type Actor%20Object%20Reference) (OtherComp :type Primitive%20Component%20Object%20Reference) (OtherBodyIndex :type Integer) (bFromSweep :type Boolean) (SweepResult :type Hit%20Result%20Structure%20%28by%20ref%29))
  (bind _asthird_person_character (Utilities|Casting|CastToThirdPersonCharacter OtherActor))
  (Variables|Default|SetRefPlayer _asthird_person_character)
  (Default|DisplayInterWidget _asthird_person_character "open" "door")
  (Variables|/Game/ThirdPersonBP/Blueprints/ThirdPersonCharacter.ThirdPersonCharacter_C|SetAreWeNearADoor? _asthird_person_character true))

(event OnComponentEndOverlap(Box)
  (params (OverlappedComponent :type Primitive%20Component%20Object%20Reference) (OtherActor :type Actor%20Object%20Reference) (OtherComp :type Primitive%20Component%20Object%20Reference) (OtherBodyIndex :type Integer))
  (bind _refplayer (Variables|Default|GetRefPlayer))
  (Default|HideInterWidget _refplayer)
  (Variables|/Game/ThirdPersonBP/Blueprints/ThirdPersonCharacter.ThirdPersonCharacter_C|SetAreWeNearADoor? _refplayer false))

(event Custom|OpenDoor
  (CallFunction|RotateDoor)
  (Components|DestroyComponent (Variables|Default|GetBox))
  (Development|SetHiddeninGame (Variables|/Game/ThirdPersonBP/Blueprints/ThirdPersonCharacter.ThirdPersonCharacter_C|GetKeyMesh (Variables|Default|GetRefPlayer)) true false))

(event Custom|RotateDoor
  (bind _doorrotationz (Timeline|DoorRotate Play)
    (:Update
      (Transformation|SetRelativeRotation (Variables|Default|GetSM_Cell_Door) (Math|Rotator|MakeRotator 0.0 0.0 _doorrotationz) false false))))

(fn ConstructionScript)