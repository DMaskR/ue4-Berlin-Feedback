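; BP_FirstKey is a key pickup actor that the player's ThirdPersonCharacter can pick up when nearby.
; On Box overlap begin, it sets the character's CanPickUpObject flag, registers itself as PickUpObject and swaps the Cube to a "can pick up" material.
; On overlap end, it clears both variables and restores the "cannot pick up" material.
; The pickup action itself is not handled here.
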(event OnComponentBeginOverlap(Box)
  (params (OverlappedComponent :type Primitive%20Component%20Object%20Reference) (OtherActor :type Actor%20Object%20Reference) (OtherComp :type Primitive%20Component%20Object%20Reference) (OtherBodyIndex :type Integer) (bFromSweep :type Boolean) (SweepResult :type Hit%20Result%20Structure%20%28by%20ref%29))
  (bind _asthird_person_character (Utilities|Casting|CastToThirdPersonCharacter OtherActor))
  (Variables|/Game/ThirdPersonBP/Blueprints/ThirdPersonCharacter.ThirdPersonCharacter_C|SetCanPickUpObject? _asthird_person_character true)
  (Variables|/Game/ThirdPersonBP/Blueprints/ThirdPersonCharacter.ThirdPersonCharacter_C|SetPickUpObject _asthird_person_character self)
  (Rendering|Material|SetMaterial (Variables|Default|GetCube) 0 "/Game/Blueprints/M_CubeMaterial_CanPickUp.M_CubeMaterial_CanPickUp"))

(event OnComponentEndOverlap(Box)
  (params (OverlappedComponent :type Primitive%20Component%20Object%20Reference) (OtherActor :type Actor%20Object%20Reference) (OtherComp :type Primitive%20Component%20Object%20Reference) (OtherBodyIndex :type Integer))
  (bind _asthird_person_character (Utilities|Casting|CastToThirdPersonCharacter OtherActor))
  (Variables|/Game/ThirdPersonBP/Blueprints/ThirdPersonCharacter.ThirdPersonCharacter_C|SetCanPickUpObject? _asthird_person_character false)
  (Variables|/Game/ThirdPersonBP/Blueprints/ThirdPersonCharacter.ThirdPersonCharacter_C|SetPickUpObject _asthird_person_character 0)
  (Rendering|Material|SetMaterial (Variables|Default|GetCube) 0 "/Game/Blueprints/M_CubeMaterial_CanNotPickUp.M_CubeMaterial_CanNotPickUp"))

(event EventBeginPlay)

(event Collision|EventActorBeginOverlap
  (params (OtherActor :type Actor%20Object%20Reference)))

(event EventTick
  (params (DeltaSeconds :type Float%20%28single-precision%29)))

(fn ConstructionScript)