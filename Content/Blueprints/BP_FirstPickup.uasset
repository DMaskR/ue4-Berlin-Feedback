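; BP_FirstPickup is a statue pickup that highlights itself and dissolves when its Dissolve event is called.
; Its box overlap registers it as the ThirdPersonCharacter's pickup target, swaps in a scanline material and shows an interaction prompt, reversing all three on exit.
; Dissolve swaps the material and starts a looping timer that raises the Opacity parameter until it reaches one, then destroys the actor.
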(event OnComponentBeginOverlap(Box)
  (params (OverlappedComponent :type Primitive%20Component%20Object%20Reference) (OtherActor :type Actor%20Object%20Reference) (OtherComp :type Primitive%20Component%20Object%20Reference) (OtherBodyIndex :type Integer) (bFromSweep :type Boolean) (SweepResult :type Hit%20Result%20Structure%20%28by%20ref%29))
  (bind _asthird_person_character (Utilities|Casting|CastToThirdPersonCharacter OtherActor))
  (Variables|/Game/Blueprints/ThirdPersonCharacter.ThirdPersonCharacter_C|SetCanPickUpObject? _asthird_person_character true)
  (Variables|/Game/Blueprints/ThirdPersonCharacter.ThirdPersonCharacter_C|SetPickUpObject _asthird_person_character self)
  (Rendering|Material|SetMaterial (Variables|Default|GetStatue) 0 "/Game/MaterialFunctionCollection/Materials/Materials/Scanline/MI_Scanline_02.MI_Scanline_02")
  (Default|DisplayInterWidget _asthird_person_character "pick up" "statue"))

(event OnComponentEndOverlap(Box)
  (params (OverlappedComponent :type Primitive%20Component%20Object%20Reference) (OtherActor :type Actor%20Object%20Reference) (OtherComp :type Primitive%20Component%20Object%20Reference) (OtherBodyIndex :type Integer))
  (bind _asthird_person_character (Utilities|Casting|CastToThirdPersonCharacter OtherActor))
  (Variables|/Game/Blueprints/ThirdPersonCharacter.ThirdPersonCharacter_C|SetCanPickUpObject? _asthird_person_character false)
  (Variables|/Game/Blueprints/ThirdPersonCharacter.ThirdPersonCharacter_C|SetPickUpObject _asthird_person_character 0)
  (Rendering|Material|SetMaterial (Variables|Default|GetStatue) 0 "/Game/MedievalDungeon/Materials/M_Statue_Hooded_Metal_Inst.M_Statue_Hooded_Metal_Inst")
  (Default|HideInterWidget _asthird_person_character))

(event Custom|Dissolve
  (Rendering|Material|SetMaterial (Variables|Default|GetStatue) 0 "/Game/Materials/M_Test_CanPickUp.M_Test_CanPickUp")
  (Utilities|Time|SetTimerbyFunctionName 0 "DecreaseOpacity" 0.01 true))

(fn ConstructionScript)

(fn DecreaseOpacity
  (Rendering|Material|SetScalarParameterValueonMaterials (Variables|Default|GetStatue) "Opacity" (Variables|Default|GetOpacity))
  (Variables|Default|SetOpacity (+ (Variables|Default|GetOpacity) 0.01))
  (if (>= (Variables|Default|GetOpacity) 1.0)
    (Utilities|Time|ClearTimerbyFunctionName 0 "DecreaseOpacity")
    (Actor|DestroyActor)))