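; BP_5th_trap is a Lights Out-style puzzle trap on a grid of twelve planes.
; TriggerPlane parses an index from the plane name and toggles that plane and its orthogonal neighbours, while Reset clears switched ones.
; Each plane has a duplicated event, so delayed transition-material swaps run independently.
; Tick polls CheckVictory, which releases the Visor's possession and spawns BP_FirstKey once all planes are switched.
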(event Custom|switchPlaneEvent
  (params (index :type Integer))
  ;[1 1 1] select switch plane event
  (switch int index
    (:0
      (CallFunction|SwitchPlane0))
    (:1
      (CallFunction|SwitchPlane1 1))
    (:2
      (CallFunction|SwitchPlane2 2))
    (:3
      (CallFunction|SwitchPlane3 3))
    (:4
      (CallFunction|SwitchPlane4 4))
    (:5
      (CallFunction|SwitchPlane5 5))
    (:6
      (CallFunction|SwitchPlane6 6))
    (:7
      (CallFunction|SwitchPlane7 7))
    (:8
      (CallFunction|SwitchPlane8 8))
    (:9
      (CallFunction|SwitchPlane9 9))
    (:10
      (CallFunction|SwitchPlane10 10))
    (:11
      (CallFunction|SwitchPlane11 11))))

(event Custom|switchPlane0
  (params (index :type Integer))
  (bind _switchtimer (Variables|Default|GetSwitchTimer))
  (bind _transitionmaterial (Variables|Default|GettransitionMaterial))
  (bind _planes (Variables|Default|GetPlanes))
  (bind _switched_planes (Variables|Default|GetSwitched_planes))
  (bind _output (Utilities|Array|Get(acopy) _planes index))
  ;[1 1 1] switch planes individually
  ;;[1 1 1] Switch plane 0
  (if (Utilities|Array|Get(acopy) (Variables|Default|GetSwitched_planes) index)
    (Rendering|Material|SetMaterial _output 0 _transitionmaterial)
    (Utilities|FlowControl|Delay _switchtimer)
    (Rendering|Material|SetMaterial _output 0 "/Engine/BasicShapes/BasicShapeMaterial.BasicShapeMaterial")
    (else
      (Rendering|Material|SetMaterial _output 0 _transitionmaterial)
      (Utilities|FlowControl|Delay _switchtimer)
      (Rendering|Material|SetMaterial _output 0 "/Game/StarterContent/Blueprints/Assets/M_LightStage_Skybox_Black.M_LightStage_Skybox_Black")))
  (Utilities|Array|SetArrayElem _switched_planes index (not (Utilities|Array|Get(acopy) _switched_planes index))))

(event Custom|switchPlane1
  (params (index :type Integer))
  (bind _switchtimer (Variables|Default|GetSwitchTimer))
  (bind _transitionmaterial (Variables|Default|GettransitionMaterial))
  (bind _planes (Variables|Default|GetPlanes))
  (bind _switched_planes (Variables|Default|GetSwitched_planes))
  (bind _output (Utilities|Array|Get(acopy) _planes index))
  ;[1 1 1] switch planes individually
  ;;[1 1 1] Switch plane 1
  (if (Utilities|Array|Get(acopy) (Variables|Default|GetSwitched_planes) index)
    (Rendering|Material|SetMaterial _output 0 _transitionmaterial)
    (Utilities|FlowControl|Delay _switchtimer)
    (Rendering|Material|SetMaterial _output 0 "/Engine/BasicShapes/BasicShapeMaterial.BasicShapeMaterial")
    (else
      (Rendering|Material|SetMaterial _output 0 _transitionmaterial)
      (Utilities|FlowControl|Delay _switchtimer)
      (Rendering|Material|SetMaterial _output 0 "/Game/StarterContent/Blueprints/Assets/M_LightStage_Skybox_Black.M_LightStage_Skybox_Black")))
  (Utilities|Array|SetArrayElem _switched_planes index (not (Utilities|Array|Get(acopy) _switched_planes index))))

(event Custom|switchPlane2
  (params (index :type Integer))
  (bind _switchtimer (Variables|Default|GetSwitchTimer))
  (bind _transitionmaterial (Variables|Default|GettransitionMaterial))
  (bind _planes (Variables|Default|GetPlanes))
  (bind _switched_planes (Variables|Default|GetSwitched_planes))
  (bind _output (Utilities|Array|Get(acopy) _planes index))
  ;[1 1 1] switch planes individually
  ;;[1 1 1] Switch plane 2
  (if (Utilities|Array|Get(acopy) (Variables|Default|GetSwitched_planes) index)
    (Rendering|Material|SetMaterial _output 0 _transitionmaterial)
    (Utilities|FlowControl|Delay _switchtimer)
    (Rendering|Material|SetMaterial _output 0 "/Engine/BasicShapes/BasicShapeMaterial.BasicShapeMaterial")
    (else
      (Rendering|Material|SetMaterial _output 0 _transitionmaterial)
      (Utilities|FlowControl|Delay _switchtimer)
      (Rendering|Material|SetMaterial _output 0 "/Game/StarterContent/Blueprints/Assets/M_LightStage_Skybox_Black.M_LightStage_Skybox_Black")))
  (Utilities|Array|SetArrayElem _switched_planes index (not (Utilities|Array|Get(acopy) _switched_planes index))))

(event Custom|switchPlane3
  (params (index :type Integer))
  (bind _switchtimer (Variables|Default|GetSwitchTimer))
  (bind _transitionmaterial (Variables|Default|GettransitionMaterial))
  (bind _planes (Variables|Default|GetPlanes))
  (bind _switched_planes (Variables|Default|GetSwitched_planes))
  (bind _output (Utilities|Array|Get(acopy) _planes index))
  ;[1 1 1] switch planes individually
  ;;[1 1 1] Switch plane 3
  (if (Utilities|Array|Get(acopy) (Variables|Default|GetSwitched_planes) index)
    (Rendering|Material|SetMaterial _output 0 _transitionmaterial)
    (Utilities|FlowControl|Delay _switchtimer)
    (Rendering|Material|SetMaterial _output 0 "/Engine/BasicShapes/BasicShapeMaterial.BasicShapeMaterial")
    (else
      (Rendering|Material|SetMaterial _output 0 _transitionmaterial)
      (Utilities|FlowControl|Delay _switchtimer)
      (Rendering|Material|SetMaterial _output 0 "/Game/StarterContent/Blueprints/Assets/M_LightStage_Skybox_Black.M_LightStage_Skybox_Black")))
  (Utilities|Array|SetArrayElem _switched_planes index (not (Utilities|Array|Get(acopy) _switched_planes index))))

(event Custom|switchPlane4
  (params (index :type Integer))
  (bind _switchtimer (Variables|Default|GetSwitchTimer))
  (bind _transitionmaterial (Variables|Default|GettransitionMaterial))
  (bind _planes (Variables|Default|GetPlanes))
  (bind _switched_planes (Variables|Default|GetSwitched_planes))
  (bind _output (Utilities|Array|Get(acopy) _planes index))
  ;[1 1 1] switch planes individually
  ;;[1 1 1] Switch plane 4
  (if (Utilities|Array|Get(acopy) (Variables|Default|GetSwitched_planes) index)
    (Rendering|Material|SetMaterial _output 0 _transitionmaterial)
    (Utilities|FlowControl|Delay _switchtimer)
    (Rendering|Material|SetMaterial _output 0 "/Engine/BasicShapes/BasicShapeMaterial.BasicShapeMaterial")
    (else
      (Rendering|Material|SetMaterial _output 0 _transitionmaterial)
      (Utilities|FlowControl|Delay _switchtimer)
      (Rendering|Material|SetMaterial _output 0 "/Game/StarterContent/Blueprints/Assets/M_LightStage_Skybox_Black.M_LightStage_Skybox_Black")))
  (Utilities|Array|SetArrayElem _switched_planes index (not (Utilities|Array|Get(acopy) _switched_planes index))))

(event Custom|switchPlane5
  (params (index :type Integer))
  (bind _switchtimer (Variables|Default|GetSwitchTimer))
  (bind _transitionmaterial (Variables|Default|GettransitionMaterial))
  (bind _planes (Variables|Default|GetPlanes))
  (bind _switched_planes (Variables|Default|GetSwitched_planes))
  (bind _output (Utilities|Array|Get(acopy) _planes index))
  ;[1 1 1] switch planes individually
  ;;[1 1 1] Switch plane 5
  (if (Utilities|Array|Get(acopy) (Variables|Default|GetSwitched_planes) index)
    (Rendering|Material|SetMaterial _output 0 _transitionmaterial)
    (Utilities|FlowControl|Delay _switchtimer)
    (Rendering|Material|SetMaterial _output 0 "/Engine/BasicShapes/BasicShapeMaterial.BasicShapeMaterial")
    (else
      (Rendering|Material|SetMaterial _output 0 _transitionmaterial)
      (Utilities|FlowControl|Delay _switchtimer)
      (Rendering|Material|SetMaterial _output 0 "/Game/StarterContent/Blueprints/Assets/M_LightStage_Skybox_Black.M_LightStage_Skybox_Black")))
  (Utilities|Array|SetArrayElem _switched_planes index (not (Utilities|Array|Get(acopy) _switched_planes index))))

(event Custom|switchPlane6
  (params (index :type Integer))
  (bind _switchtimer (Variables|Default|GetSwitchTimer))
  (bind _transitionmaterial (Variables|Default|GettransitionMaterial))
  (bind _planes (Variables|Default|GetPlanes))
  (bind _switched_planes (Variables|Default|GetSwitched_planes))
  (bind _output (Utilities|Array|Get(acopy) _planes index))
  ;[1 1 1] switch planes individually
  ;;[1 1 1] Switch plane 6
  (if (Utilities|Array|Get(acopy) (Variables|Default|GetSwitched_planes) index)
    (Rendering|Material|SetMaterial _output 0 _transitionmaterial)
    (Utilities|FlowControl|Delay _switchtimer)
    (Rendering|Material|SetMaterial _output 0 "/Engine/BasicShapes/BasicShapeMaterial.BasicShapeMaterial")
    (else
      (Rendering|Material|SetMaterial _output 0 _transitionmaterial)
      (Utilities|FlowControl|Delay _switchtimer)
      (Rendering|Material|SetMaterial _output 0 "/Game/StarterContent/Blueprints/Assets/M_LightStage_Skybox_Black.M_LightStage_Skybox_Black")))
  (Utilities|Array|SetArrayElem _switched_planes index (not (Utilities|Array|Get(acopy) _switched_planes index))))

(event Custom|switchPlane7
  (params (index :type Integer))
  (bind _switched_planes (Variables|Default|GetSwitched_planes))
  (bind _switchtimer (Variables|Default|GetSwitchTimer))
  (bind _transitionmaterial (Variables|Default|GettransitionMaterial))
  (bind _planes (Variables|Default|GetPlanes))
  (bind _output (Utilities|Array|Get(acopy) _planes index))
  ;[1 1 1] switch planes individually
  ;;[1 1 1] Switch plane 7
  (if (Utilities|Array|Get(acopy) (Variables|Default|GetSwitched_planes) index)
    (Rendering|Material|SetMaterial _output 0 _transitionmaterial)
    (Utilities|FlowControl|Delay _switchtimer)
    (Rendering|Material|SetMaterial _output 0 "/Engine/BasicShapes/BasicShapeMaterial.BasicShapeMaterial")
    (else
      (Rendering|Material|SetMaterial _output 0 _transitionmaterial)
      (Utilities|FlowControl|Delay _switchtimer)
      (Rendering|Material|SetMaterial _output 0 "/Game/StarterContent/Blueprints/Assets/M_LightStage_Skybox_Black.M_LightStage_Skybox_Black")))
  (Utilities|Array|SetArrayElem _switched_planes index (not (Utilities|Array|Get(acopy) _switched_planes index))))

(event Custom|switchPlane8
  (params (index :type Integer))
  (bind _planes (Variables|Default|GetPlanes))
  (bind _switched_planes (Variables|Default|GetSwitched_planes))
  (bind _switchtimer (Variables|Default|GetSwitchTimer))
  (bind _transitionmaterial (Variables|Default|GettransitionMaterial))
  (bind _output (Utilities|Array|Get(acopy) _planes index))
  ;[1 1 1] switch planes individually
  ;;[1 1 1] Switch plane 8
  (if (Utilities|Array|Get(acopy) (Variables|Default|GetSwitched_planes) index)
    (Rendering|Material|SetMaterial _output 0 _transitionmaterial)
    (Utilities|FlowControl|Delay _switchtimer)
    (Rendering|Material|SetMaterial _output 0 "/Engine/BasicShapes/BasicShapeMaterial.BasicShapeMaterial")
    (else
      (Rendering|Material|SetMaterial _output 0 _transitionmaterial)
      (Utilities|FlowControl|Delay _switchtimer)
      (Rendering|Material|SetMaterial _output 0 "/Game/StarterContent/Blueprints/Assets/M_LightStage_Skybox_Black.M_LightStage_Skybox_Black")))
  (Utilities|Array|SetArrayElem _switched_planes index (not (Utilities|Array|Get(acopy) _switched_planes index))))

(event Custom|switchPlane9
  (params (index :type Integer))
  (bind _planes (Variables|Default|GetPlanes))
  (bind _switched_planes (Variables|Default|GetSwitched_planes))
  (bind _switchtimer (Variables|Default|GetSwitchTimer))
  (bind _transitionmaterial (Variables|Default|GettransitionMaterial))
  (bind _output (Utilities|Array|Get(acopy) _planes index))
  ;[1 1 1] switch planes individually
  ;;[1 1 1] Switch plane 9
  (if (Utilities|Array|Get(acopy) (Variables|Default|GetSwitched_planes) index)
    (Rendering|Material|SetMaterial _output 0 _transitionmaterial)
    (Utilities|FlowControl|Delay _switchtimer)
    (Rendering|Material|SetMaterial _output 0 "/Engine/BasicShapes/BasicShapeMaterial.BasicShapeMaterial")
    (else
      (Rendering|Material|SetMaterial _output 0 _transitionmaterial)
      (Utilities|FlowControl|Delay _switchtimer)
      (Rendering|Material|SetMaterial _output 0 "/Game/StarterContent/Blueprints/Assets/M_LightStage_Skybox_Black.M_LightStage_Skybox_Black")))
  (Utilities|Array|SetArrayElem _switched_planes index (not (Utilities|Array|Get(acopy) _switched_planes index))))

(event Custom|switchPlane10
  (params (index :type Integer))
  (bind _planes (Variables|Default|GetPlanes))
  (bind _switched_planes (Variables|Default|GetSwitched_planes))
  (bind _switchtimer (Variables|Default|GetSwitchTimer))
  (bind _transitionmaterial (Variables|Default|GettransitionMaterial))
  (bind _output (Utilities|Array|Get(acopy) _planes index))
  ;[1 1 1] switch planes individually
  ;;[1 1 1] Switch plane 10
  (if (Utilities|Array|Get(acopy) (Variables|Default|GetSwitched_planes) index)
    (Rendering|Material|SetMaterial _output 0 _transitionmaterial)
    (Utilities|FlowControl|Delay _switchtimer)
    (Rendering|Material|SetMaterial _output 0 "/Engine/BasicShapes/BasicShapeMaterial.BasicShapeMaterial")
    (else
      (Rendering|Material|SetMaterial _output 0 _transitionmaterial)
      (Utilities|FlowControl|Delay _switchtimer)
      (Rendering|Material|SetMaterial _output 0 "/Game/StarterContent/Blueprints/Assets/M_LightStage_Skybox_Black.M_LightStage_Skybox_Black")))
  (Utilities|Array|SetArrayElem _switched_planes index (not (Utilities|Array|Get(acopy) _switched_planes index))))

(event Custom|switchPlane11
  (params (index :type Integer))
  (bind _planes (Variables|Default|GetPlanes))
  (bind _switched_planes (Variables|Default|GetSwitched_planes))
  (bind _switchtimer (Variables|Default|GetSwitchTimer))
  (bind _transitionmaterial (Variables|Default|GettransitionMaterial))
  (bind _output (Utilities|Array|Get(acopy) _planes index))
  ;[1 1 1] switch planes individually
  ;;[1 1 1] Switch plane 11
  (if (Utilities|Array|Get(acopy) (Variables|Default|GetSwitched_planes) index)
    (Rendering|Material|SetMaterial _output 0 _transitionmaterial)
    (Utilities|FlowControl|Delay _switchtimer)
    (Rendering|Material|SetMaterial _output 0 "/Engine/BasicShapes/BasicShapeMaterial.BasicShapeMaterial")
    (else
      (Rendering|Material|SetMaterial _output 0 _transitionmaterial)
      (Utilities|FlowControl|Delay _switchtimer)
      (Rendering|Material|SetMaterial _output 0 "/Game/StarterContent/Blueprints/Assets/M_LightStage_Skybox_Black.M_LightStage_Skybox_Black")))
  (Utilities|Array|SetArrayElem _switched_planes index (not (Utilities|Array|Get(acopy) _switched_planes index))))

(event EventBeginPlay
  ;[1 1 1] put planes into array
  (Variables|Default|SetPlanes (Utilities|Array|MakeArray (Variables|Default|GetPlane_0) (Variables|Default|GetPlane_1) (Variables|Default|GetPlane_2) (Variables|Default|GetPlane_3) (Variables|Default|GetPlane_4) (Variables|Default|GetPlane_5) (Variables|Default|GetPlane_6) (Variables|Default|GetPlane_7) (Variables|Default|GetPlane_8) (Variables|Default|GetPlane_9) (Variables|Default|GetPlane_10) (Variables|Default|GetPlane_11))))

(event EventTick
  (params (DeltaSeconds :type Float%20%28single-precision%29))
  (if (not (Variables|Default|Getwon))
    (CallFunction|CheckVictory)))

(fn ConstructionScript)

(fn TriggerPlane
  (params (planeName :type String) (Visor :type BP%20Plane%20Visor%20Object%20Reference))
  (bind _returnvalue (Utilities|String|ParseIntoArray planeName "_"))
  (Variables|Default|SetVisor Visor)
  (bind _output_get (LocalVariables|SetPlaneIndex (Math|Conversions|ToInteger(Byte) (Utilities|Array|Get(acopy) _returnvalue (- (Utilities|Array|Length _returnvalue) 1)))))
  (CallFunction|SwitchPlaneEvent _output_get)
  (if (> (Math|Integer|%(Integer) _output_get 4) 0)
    (CallFunction|SwitchPlaneEvent (- (LocalVariables|GetPlaneIndex) 1)))
  (if (< (Math|Integer|%(Integer) _output_get 4) 3)
    (CallFunction|SwitchPlaneEvent (+ (LocalVariables|GetPlaneIndex) 1)))
  (if (> (Math|Integer|%(Integer) (- _output_get (Math|Integer|%(Integer) _output_get 4)) 3) 0)
    (CallFunction|SwitchPlaneEvent (- (LocalVariables|GetPlaneIndex) 4)))
  (if (< (Math|Integer|%(Integer) (- _output_get (Math|Integer|%(Integer) _output_get 4)) 3) 2)
    (CallFunction|SwitchPlaneEvent (+ (LocalVariables|GetPlaneIndex) 4))))

(fn SwitchPlane
  (params (Index :type Integer))
  (bind _planes (Variables|Default|GetPlanes))
  (bind _switched_planes (Variables|Default|GetSwitched_planes))
  (bind _output (Utilities|Array|Get(acopy) _planes Index))
  (if (Utilities|Array|Get(acopy) (Variables|Default|GetSwitched_planes) Index)
    (Rendering|Material|SetMaterial _output 0 "/Game/MaterialFunctionCollection/Materials/Materials/Dissolve/MI_Dissolve_01.MI_Dissolve_01")
    (else
      (Rendering|Material|SetMaterial _output 0 "/Game/MaterialFunctionCollection/Materials/Materials/Scanline/M_Scanline.M_Scanline")))
  (Utilities|Array|SetArrayElem _switched_planes Index (not (Utilities|Array|Get(acopy) _switched_planes Index))))

(fn CheckVictory
  (for _array_element (Variables|Default|GetSwitched_planes)
    (if (not _array_element)
      (LocalVariables|SetIsAnyWhite true)))
  (if (not (LocalVariables|GetIsAnyWhite))
    (Default|ReleasePossession (Variables|Default|GetVisor))
    (Game|SpawnActorfromClass "/Game/Blueprints/BP_FirstKey.BP_FirstKey_C" (Transformation|GetWorldTransform (Variables|Default|GetBox)) "Undefined" 0 0)
    (Variables|Default|Setwon true)))

(fn Reset
  (for (_array_element _array_index) (Variables|Default|GetSwitched_planes)
    (if _array_element
      (CallFunction|SwitchPlaneEvent _array_index))))