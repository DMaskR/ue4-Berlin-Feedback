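; Rotatable gargoyle statue for a puzzle, starting at a random yaw of 90, 180 or 270, rolled separately for the mesh and ResultRotation.
; Its overlap box shows the character's rotate prompt and registers the statue on that character.
; RotateStatue plays a timeline that offsets the current yaw while flagging the character as rotating.
; When finished, it stores ResultRotation and asks the parent BP_CheckStatue to check for a win.
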(event OnComponentBeginOverlap(Box)
  (params (OverlappedComponent :type Primitive%20Component%20Object%20Reference) (OtherActor :type Actor%20Object%20Reference) (OtherComp :type Primitive%20Component%20Object%20Reference) (OtherBodyIndex :type Integer) (bFromSweep :type Boolean) (SweepResult :type Hit%20Result%20Structure%20%28by%20ref%29))
  (bind _asthird_person_character (Utilities|Casting|CastToThirdPersonCharacter OtherActor))
  (Development|PrintString "Hello player overlapping")
  (Variables|Default|SetRefThirdPersonCharacter _asthird_person_character)
  (Default|DisplayInterWidget _asthird_person_character "rotate" "statue")
  (Variables|/Game/Blueprints/ThirdPersonCharacter.ThirdPersonCharacter_C|SetAre%20We%20Near%20AStatue? _asthird_person_character true)
  (Variables|/Game/Blueprints/ThirdPersonCharacter.ThirdPersonCharacter_C|SetStatueObject _asthird_person_character self))

(event OnComponentEndOverlap(Box)
  (params (OverlappedComponent :type Primitive%20Component%20Object%20Reference) (OtherActor :type Actor%20Object%20Reference) (OtherComp :type Primitive%20Component%20Object%20Reference) (OtherBodyIndex :type Integer))
  (bind _refthirdpersoncharacter (Variables|Default|GetRefThirdPersonCharacter))
  (Default|HideInterWidget _refthirdpersoncharacter)
  (Variables|/Game/Blueprints/ThirdPersonCharacter.ThirdPersonCharacter_C|SetAre%20We%20Near%20AStatue? _refthirdpersoncharacter false)
  (Variables|/Game/Blueprints/ThirdPersonCharacter.ThirdPersonCharacter_C|SetStatueObject _refthirdpersoncharacter self))

(event Custom|RotateAnimation
  (bind _refthirdpersoncharacter (Variables|Default|GetRefThirdPersonCharacter))
  (Variables|/Game/Blueprints/ThirdPersonCharacter.ThirdPersonCharacter_C|SetStatueInRotation _refthirdpersoncharacter true)
  (Variables|Components|SetStatueRotation (.Yaw (Math|Rotator|BreakRotator (Variables|/Script/Engine.SceneComponent|GetRelativeRotation (Variables|Default|GetGargoyle)))))
  (bind _statuerotationz (Timeline|Timeline_1 PlayFromStart)
    (:Update
      (Transformation|SetRelativeRotation (Variables|Default|GetGargoyle) (Math|Rotator|MakeRotator 0.0 0.0 (+ _statuerotationz (Variables|Components|GetStatueRotation))) false false))
    (:Finished
      (Variables|Components|SetResultRotation (Math|Rotator|MakeRotator 0.0 0.0 (+ _statuerotationz (Variables|Components|GetStatueRotation))))
      (Variables|/Game/Blueprints/ThirdPersonCharacter.ThirdPersonCharacter_C|SetStatueInRotation _refthirdpersoncharacter false)
      (Development|PrintString (Utilities|String|ToString(Float) (.Yaw (Math|Rotator|BreakRotator (Variables|/Script/Engine.SceneComponent|GetRelativeRotation (Variables|Default|GetGargoyle))))) true true "(R=1.000000,G=0.860128,B=0.000000,A=1.000000)")
      (bind _asbp_check_statue (Utilities|Casting|CastToBP_CheckStatue (Variables|Components|GetTheParrentActor)))
      (Default|CheckStatueWin _asbp_check_statue))))

(event Custom|RotateStatue
  (Development|PrintString "Launch rotation")
  (CallFunction|RotateAnimation))

(event EventBeginPlay
  (bind _gargoyle (Variables|Default|GetGargoyle))
  (bind _result (Utilities|Set|ToArray (Utilities|Set|MakeSet 9e+01 1.8e+02 2.7e+02)))
  (Development|PrintString (Utilities|String|ToString(Float) (.OutItem (Utilities|Array|Random _result))) true true "(R=0.000000,G=0.098422,B=1.000000,A=1.000000)")
  (Components|MoveComponentTo _gargoyle (Variables|/Script/Engine.SceneComponent|GetRelativeLocation _gargoyle) (Math|Rotator|MakeRotator 0.0 0.0 (.OutItem (Utilities|Array|Random _result))) true true 0.0 false)
  (Variables|Components|SetResultRotation (Math|Rotator|MakeRotator 0.0 0.0 (.OutItem (Utilities|Array|Random _result)))))

(fn ConstructionScript)