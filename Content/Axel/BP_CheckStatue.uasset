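; BP_CheckStatue checks whether a four-statue rotation puzzle is solved.
; Its CheckStatueWin event casts four target actors to BP_StatuePuzle and prints each one's ResultRotation yaw for debugging.
; Success requires every ResultRotation to be zero within a small tolerance, and currently only prints a confirmation message.
; Any failed cast prints a shared error message.
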(event Custom|CheckStatueWin
  (bind _asstatue_puzle (Utilities|Casting|CastToBP_StatuePuzle (Variables|Default|GetTargetActor1))
    (:then
      (bind _asstatue_puzle_2 (Utilities|Casting|CastToBP_StatuePuzle (Variables|Default|GetTargetActor2))
        (:then
          (bind _asstatue_puzle_3 (Utilities|Casting|CastToBP_StatuePuzle (Variables|Default|GetTargetActor3))
            (:then
              (bind _asstatue_puzle_4 (Utilities|Casting|CastToBP_StatuePuzle (Variables|Default|GetTargetActor4))
                (:then
                  (Development|PrintString (Utilities|String|Append "Statue 1:" (Utilities|String|ToString(Float) (.Yaw (Math|Rotator|BreakRotator (Variables|/Game/Axel/BP_StatuePuzle.BP_StatuePuzle_C|GetResultRotation _asstatue_puzle))))) true true "(R=1.000000,G=0.000000,B=0.353798,A=1.000000)")
                  (Development|PrintString (Utilities|String|Append "Statue 2:" (Utilities|String|ToString(Float) (.Yaw (Math|Rotator|BreakRotator (Variables|/Game/Axel/BP_StatuePuzle.BP_StatuePuzle_C|GetResultRotation _asstatue_puzle_2))))) true true "(R=1.000000,G=0.000000,B=0.353798,A=1.000000)")
                  (Development|PrintString (Utilities|String|Append "Statue 3:" (Utilities|String|ToString(Float) (.Yaw (Math|Rotator|BreakRotator (Variables|/Game/Axel/BP_StatuePuzle.BP_StatuePuzle_C|GetResultRotation _asstatue_puzle_3))))) true true "(R=1.000000,G=0.000000,B=0.353798,A=1.000000)")
                  (Development|PrintString (Utilities|String|Append "Statue 4:" (Utilities|String|ToString(Float) (.Yaw (Math|Rotator|BreakRotator (Variables|/Game/Axel/BP_StatuePuzle.BP_StatuePuzle_C|GetResultRotation _asstatue_puzle_4))))) true true "(R=1.000000,G=0.000000,B=0.353798,A=1.000000)")
                  (if (Math|Rotator|Equal(Rotator) (Variables|/Game/Axel/BP_StatuePuzle.BP_StatuePuzle_C|GetResultRotation _asstatue_puzle) "0, 0, 0" 0.01)
                    (if (Math|Rotator|Equal(Rotator) (Variables|/Game/Axel/BP_StatuePuzle.BP_StatuePuzle_C|GetResultRotation _asstatue_puzle_2) "0, 0, 0" 0.01)
                      (if (Math|Rotator|Equal(Rotator) (Variables|/Game/Axel/BP_StatuePuzle.BP_StatuePuzle_C|GetResultRotation _asstatue_puzle_3) "0, 0, 0" 0.01)
                        (if (Math|Rotator|Equal(Rotator) (Variables|/Game/Axel/BP_StatuePuzle.BP_StatuePuzle_C|GetResultRotation _asstatue_puzle_4) "0, 0, 0" 0.01)
                          (Development|PrintString "all the statue are in the correct position"))))))
                (:CastFailed
                  (Development|PrintString "cast faild" true true "(R=0.672191,G=0.000000,B=1.000000,A=1.000000)" :!label _label))))
            (:CastFailed
              (goto _label))))
        (:CastFailed
          (goto _label))))
    (:CastFailed
      (goto _label))))

(fn ConstructionScript)