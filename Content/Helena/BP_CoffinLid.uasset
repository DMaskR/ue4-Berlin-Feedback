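; Interactable coffin whose lid slides open once, in a direction that depends on the side given to OpenCoffin.
; Front and Back trigger overlaps show an "open coffin" prompt on the ThirdPersonCharacter while closed, passing it a self reference, a nearby flag and which side it is on.
; Leaving either trigger hides the prompt and clears the nearby flag, but keeps the coffin reference.
; OpenCoffin eases the lid along relative Y with MoveComponentTo, then sets IsOpen.
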(event OnComponentBeginOverlap(Back)
  (params (OverlappedComponent :type Primitive%20Component%20Object%20Reference) (OtherActor :type Actor%20Object%20Reference) (OtherComp :type Primitive%20Component%20Object%20Reference) (OtherBodyIndex :type Integer) (bFromSweep :type Boolean) (SweepResult :type Hit%20Result%20Structure%20%28by%20ref%29))
  (if (not (Variables|Default|GetIsOpen))
    (bind _asthird_person_character (Utilities|Casting|CastToThirdPersonCharacter OtherActor))
    (Variables|Default|SetRefPlayerFixed _asthird_person_character)
    (Default|DisplayInterWidget _asthird_person_character "open" "coffin")
    (Variables|/Game/Blueprints/ThirdPersonCharacter.ThirdPersonCharacter_C|SetAreWeNearACoffin? _asthird_person_character true)
    (Variables|/Game/Blueprints/ThirdPersonCharacter.ThirdPersonCharacter_C|SetCoffinRef _asthird_person_character self)
    (Variables|/Game/Blueprints/ThirdPersonCharacter.ThirdPersonCharacter_C|SetIsInFrontOfCoffin _asthird_person_character false)
    (Development|PrintString (Utilities|GetObjectName (Variables|/Game/Blueprints/ThirdPersonCharacter.ThirdPersonCharacter_C|GetCoffinRef _asthird_person_character)))))

(event OnComponentEndOverlap(Back)
  (params (OverlappedComponent :type Primitive%20Component%20Object%20Reference) (OtherActor :type Actor%20Object%20Reference) (OtherComp :type Primitive%20Component%20Object%20Reference) (OtherBodyIndex :type Integer))
  (bind _refplayerfixed (Variables|Default|GetRefPlayerFixed))
  (Default|HideInterWidget _refplayerfixed)
  (Variables|/Game/Blueprints/ThirdPersonCharacter.ThirdPersonCharacter_C|SetAreWeNearACoffin? _refplayerfixed false)
  (Variables|/Game/Blueprints/ThirdPersonCharacter.ThirdPersonCharacter_C|SetCoffinRef _refplayerfixed self))

(event OnComponentBeginOverlap(Front)
  (params (OverlappedComponent :type Primitive%20Component%20Object%20Reference) (OtherActor :type Actor%20Object%20Reference) (OtherComp :type Primitive%20Component%20Object%20Reference) (OtherBodyIndex :type Integer) (bFromSweep :type Boolean) (SweepResult :type Hit%20Result%20Structure%20%28by%20ref%29))
  (if (not (Variables|Default|GetIsOpen))
    (bind _asthird_person_character (Utilities|Casting|CastToThirdPersonCharacter OtherActor))
    (bind _output_get (Variables|Default|SetRefPlayerFixed _asthird_person_character))
    (Default|DisplayInterWidget _output_get "open" "coffin")
    (Variables|/Game/Blueprints/ThirdPersonCharacter.ThirdPersonCharacter_C|SetAreWeNearACoffin? _output_get true)
    (Variables|/Game/Blueprints/ThirdPersonCharacter.ThirdPersonCharacter_C|SetCoffinRef _output_get self)
    (Variables|/Game/Blueprints/ThirdPersonCharacter.ThirdPersonCharacter_C|SetIsInFrontOfCoffin _output_get true)))

(event OnComponentEndOverlap(Front)
  (params (OverlappedComponent :type Primitive%20Component%20Object%20Reference) (OtherActor :type Actor%20Object%20Reference) (OtherComp :type Primitive%20Component%20Object%20Reference) (OtherBodyIndex :type Integer))
  (bind _refplayerfixed (Variables|Default|GetRefPlayerFixed))
  (Default|HideInterWidget _refplayerfixed)
  (Variables|/Game/Blueprints/ThirdPersonCharacter.ThirdPersonCharacter_C|SetAreWeNearACoffin? _refplayerfixed false)
  (Variables|/Game/Blueprints/ThirdPersonCharacter.ThirdPersonCharacter_C|SetCoffinRef _refplayerfixed self))

(event Custom|OpenCoffin
  (params (fromFront :type Boolean))
  (bind _lid (Variables|Default|GetLid))
  (bind _relativelocation (Variables|/Script/Engine.SceneComponent|GetRelativeLocation _lid))
  (bind _relativerotation (Variables|/Script/Engine.SceneComponent|GetRelativeRotation _lid))
  (if (not (Variables|Default|GetIsOpen))
    (if fromFront
      (Components|MoveComponentTo _lid (Math|Vector|MakeVector (.x _relativelocation) (- (.y _relativelocation) 3e+01) (.z _relativelocation)) _relativerotation true true 1.5 false)
      (Variables|Default|SetIsOpen true)
      (else
        (Components|MoveComponentTo _lid (Math|Vector|MakeVector (.x _relativelocation) (+ (.y _relativelocation) 3e+01) (.z _relativelocation)) _relativerotation true true 1.5 false)
        (Variables|Default|SetIsOpen true)))))

(event EventBeginPlay)

(event Collision|EventActorBeginOverlap
  (params (OtherActor :type Actor%20Object%20Reference)))

(event EventTick
  (params (DeltaSeconds :type Float%20%28single-precision%29)))

(fn ConstructionScript)